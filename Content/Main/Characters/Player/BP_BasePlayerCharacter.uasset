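; Base player character Blueprint that handles input for sprinting, walk toggling, crouching and dodge rolling.
; Sprint and walk inputs switch a movement speed mode that sets max walk speed, while crouch alternates through a FlipFlop when not falling.
; Roll is gated by the StateManager action, montage playback and falling checks, then turns the actor to camera yaw, plays the montage and resets the action to Idle on completion.
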(event Input|ActionEvents|InputActionSpriting
  (params (Key :type Key%20Structure :default "None"))
  (:Pressed
    (CallFunction|SetMovementSpeedMode "NewEnumerator2"))
  (:Released
    (if (Utilities|Enum|Equal(Enum) (CallFunction|GetCurrentSpeedMode) "NewEnumerator2")
      (CallFunction|SetMovementSpeedMode "NewEnumerator1"))))

(event Input|ActionEvents|InputActionToggleWalk
  (params (Key :type Key%20Structure :default "None"))
  (:Pressed
    (if (Utilities|Enum|NotEqual(Enum) (CallFunction|GetCurrentSpeedMode) "NewEnumerator0")
      (CallFunction|SetMovementSpeedMode "NewEnumerator0")
      (else
        (CallFunction|SetMovementSpeedMode "NewEnumerator1")))))

(event Input|ActionEvents|InputActionCrounch
  (params (Key :type Key%20Structure :default "None"))
  (:Pressed
    (if (not (AI|Components|NavMovement|IsFalling (Variables|Character|GetCharacterMovement)))
      (Utilities|FlowControl|FlipFlop
        (:A
          (Character|Crouch))
        (:B
          (Character|UnCrouch))))))

(event Input|ActionEvents|InputActionRoll
  (params (Key :type Key%20Structure :default "None"))
  (:Pressed
    (if (CallFunction|CanPerformRoll)
      (Class|StateManagerComponent|SetAction (Variables|Default|GetStateManager) "(TagName=\"Character.Actions.Dodge\")")
      (CallFunction|CalculateCameraDirection)
      (Animation|Montage|PlayMontage (Variables|Character|GetMesh) "/Game/SwordAnimationPack/Animations/Roll/Game/SwordAnimationPack/Animations/Roll/Roll_F_Montage.Roll_F_Montage"
        (:OnCompleted
          (Class|StateManagerComponent|SetAction (Variables|Default|GetStateManager) "(TagName=\"Character.Actions.Idle\")"))))))

(fn ConstructionScript)

(fn SetMovementSpeedMode
  (params (NewSpeedMode :type Enum_MovementSpeedMode%20Enum :default "NewEnumerator0"))
  (if (Utilities|Enum|NotEqual(Enum) NewSpeedMode (Variables|Default|GetMovementSpeedMode))
    (bind _output_get (Variables|Default|SetMovementSpeedMode NewSpeedMode))
    (switch Utilities|FlowControl|Switch|SwitchonEnum_MovementSpeedMode _output_get
      (:NewEnumerator0
        (Variables|/Script/Engine.CharacterMovementComponent|SetMaxWalkSpeed (Variables|Character|GetCharacterMovement) (Variables|MovementSpeed|GetWalkingSpeed)))
      (:NewEnumerator1
        (Variables|/Script/Engine.CharacterMovementComponent|SetMaxWalkSpeed (Variables|Character|GetCharacterMovement) (Variables|MovementSpeed|GetJoggingSpeed)))
      (:NewEnumerator2
        (Variables|/Script/Engine.CharacterMovementComponent|SetMaxWalkSpeed (Variables|Character|GetCharacterMovement) (Variables|MovementSpeed|GetSpritingSpeed))))))

(fn GetCurrentSpeedMode
  (return (Variables|Default|GetMovementSpeedMode)))

(fn IsIdle
  (return (not (Animation|Montage|MontageIsPlaying (Components|SkeletalMesh|GetAnimInstance (Variables|Character|GetMesh)) 0))))

(fn CalculateCameraDirection
  (bind _returnvalue (Transformation|GetActorRotation))
  (bind _returnvalue_2 (Transformation|GetActorLocation))
  (Transformation|SetActorRotation (Math|Rotator|MakeRotator (.roll _returnvalue) (.pitch _returnvalue) (.yaw (Math|Rotator|FindLookatRotation _returnvalue_2 (+ _returnvalue_2 (* (Math|Vector|GetForwardVector (Variables|Default|GetFollowCamera)) 1e+03)))))))

(fn CanPerformRoll
  (return (Math|Boolean|ANDBoolean (not (Class|StateManagerComponent|IsCurrentActionEqualtoSAny (Variables|Default|GetStateManager) "(GameplayTags=((TagName=\"Character.Actions.EnterCombat\"),(TagName=\"Character.Actions.ExitCombat\"),(TagName=\"Character.Actions.Attack.ChargerdAttack\"),(TagName=\"Character.Actions.Attack.HeavyAttack\"),(TagName=\"Character.Actions.Attack.LigthAttack\"),(TagName=\"Character.Actions.Dodge\")))")) (CallFunction|IsIdle) (not (AI|Components|NavMovement|IsFalling (Variables|Character|GetCharacterMovement))))))